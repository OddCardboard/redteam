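; Player character for a 2D platformer, handling movement, jumping, health and respawn.
; Enhanced Input drives movement along X, flips control rotation to face travel direction, and triggers jumps.
; Damage grants a brief invulnerability window, or calls the GM_2DPlatformer respawn event when health runs out; BeginPlay gives that game mode the spawn transform.
; Tick picks idle, run or jump flipbooks from movement state.
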(event `self.ReceiveTick`
  (params (DeltaSeconds :type "Float (single-precision)"))
  (`self.UpdateAnimation`))

(event `self.ReceiveBeginPlay`
  ; EventBeginPlay
  ;;[1 0.8478 0.1094 0.5] NathenReed: Logic to set intial spawn
  (bind _asgm_2dplatformer (cast `/Game/Blueprints/GM_2DPlatformer` (`GameplayStatics.GetGameMode`)))
  (set `/Game/Blueprints/GM_2DPlatformer.SpawnTransform` (`self.GetTransform`) _asgm_2dplatformer)
  (bind _asplayer_controller (cast `PlayerController` (`self.GetController`)))
  (`EnhancedInputSubsystemInterface.AddMappingContext` (pcsubsystem `EnhancedInputLocalPlayerSubsystem` _asplayer_controller) "/Game/Input/IMC_Platforming.IMC_Platforming" 0 (struct)))

(event `EnhancedInput|/Game/Input/Actions/IA_Move`
  (params (ActionValue :type "Float (double-precision)") (ElapsedSeconds :type "Float (double-precision)") (TriggeredSeconds :type "Float (double-precision)") (InputAction :type "InputAction Object Reference" :default "/Game/Input/Actions/IA_Move.IA_Move"))
  ; Player Movement
  (:`Triggered`
    (`self.AddMovementInput` (1.0 0.0 0.0) ActionValue)
    (`Controller.SetControlRotation` (`self.GetController`) (select `bool` (> ActionValue 0.0) :`false` (`KismetMathLibrary.MakeRotator` 0.0 0.0 180.0) :`true` (`KismetMathLibrary.MakeRotator` 0.0)))))

(event `Add Health`
  (bind _health (`self.Health`))
  ;[0.4072 0.3467 0.04374] Add Health (ToDo: Please make a health Widget... make sure that health widget variable updates anytime this is called.)
  (if (not (>= _health (`self.MaxHealth`)))
    (set `self.Health` (+ _health 1.0))))

(event `EnhancedInput|/Game/Input/Actions/IA_Jump`
  (params (ActionValue :type Boolean) (ElapsedSeconds :type "Float (double-precision)") (TriggeredSeconds :type "Float (double-precision)") (InputAction :type "InputAction Object Reference" :default "/Game/Input/Actions/IA_Jump.IA_Jump"))
  ; Jumping
  ;;[0.06125 0.001214 0] ToDo: Please implement long/short jumping and Double jump
  (:`Started`
    (`self.Jump`))
  (:`Completed`
    (`self.StopJumping`)))

(event `self.ReceiveAnyDamage`
  (params (Damage :type "Float (single-precision)") (DamageType :type "DamageType Object Reference") (InstigatedBy :type "Controller Object Reference") (DamageCauser :type "Actor Object Reference"))
  ;[0.4072 0.3467 0.04374] Lose Health (Nathen Reed note: Cedrick, feel free to change this around as you like this is temp logic for taking damage on player)
  (if (not (`self.IsShielded`))
    (set `self.Health` (- (`self.Health`) Damage))
    (if (<= (`self.Health`) 0.0)
      (bind _asgm_2dplatformer (cast `/Game/Blueprints/GM_2DPlatformer` (`GameplayStatics.GetGameMode`)))
      (`/Game/Blueprints/GM_2DPlatformer.RespawnEvent` _asgm_2dplatformer self)
      (else
        (set `self.IsShielded` true)
        (`KismetSystemLibrary.Delay` 1.0)
        (set `self.IsShielded` false)))))

(fn `UpdateAnimation`
  (if (`NavMovementComponent.IsMovingOnGround` (`self.CharacterMovement`))
    (if (> (`KismetMathLibrary.VSize` (`self.GetVelocity`)) 0.0)
      (`PaperFlipbookComponent.SetFlipbook` (`self.Sprite`) "/Game/Blueprints/Characters/FB_Player_Run.FB_Player_Run")
      (else
        (`PaperFlipbookComponent.SetFlipbook` (`self.Sprite`) "/Game/Blueprints/Characters/FB_Player_Idle.FB_Player_Idle")))
    (elif (`NavMovementComponent.IsFalling` (`self.CharacterMovement`))
      (`PaperFlipbookComponent.SetFlipbook` (`self.Sprite`) "/Game/Blueprints/Characters/FB_Player_Jump.FB_Player_Jump"))))

(fn `UserConstructionScript`)