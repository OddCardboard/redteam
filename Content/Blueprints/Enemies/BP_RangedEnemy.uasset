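; BP_RangedEnemy is a 2D patrolling enemy that throws projectiles at the player and can be killed by damage, including stomps.
; It walks until wall or ledge trigger overlaps flip it around.
; While the player is inside AttackCheck, it stops, switches to a throwing flipbook, and uses looping timers to face, aim and fire.
; StompBox applies damage and launches the player upward; UpdateHealth is an empty stub.
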(event `self.WallCheck.OnComponentBeginOverlap`
  (params (OverlappedComponent :type "PrimitiveComponent Object Reference") (OtherActor :type "Actor Object Reference") (OtherComp :type "PrimitiveComponent Object Reference") (OtherBodyIndex :type Integer) (bFromSweep :type Boolean) (SweepResult :type "HitResult Structure (by ref)"))
  ; Terrain Checking
  (`self.TurnChar`))

(event `self.ReceiveTick`
  (params (DeltaSeconds :type "Float (single-precision)"))
  ; Forward Movement
  (if (`self.NotShooting`)
    (`self.AddMovementInput` (`self.GetActorForwardVector`) -1.0)))

(event `self.LedgeCheck.OnComponentEndOverlap`
  (params (OverlappedComponent :type "PrimitiveComponent Object Reference") (OtherActor :type "Actor Object Reference") (OtherComp :type "PrimitiveComponent Object Reference") (OtherBodyIndex :type Integer))
  ; Terrain Checking
  (`self.TurnChar`))

(event `TurnToPlayer`
  (bind _returnvalue_x (`KismetMathLibrary.BreakVector` (`self.K2_GetActorLocation`)))
  (bind _returnvalue_x_2 (`KismetMathLibrary.BreakVector` (`self.GetActorForwardVector`)))
  (bind _returnvalue_x_3 (`KismetMathLibrary.BreakVector` (`self.K2_GetActorLocation` (`GameplayStatics.GetPlayerCharacter` 0))))
  (bind _returnvalue (== _returnvalue_x_2 1.0))
  ; Follow Player
  (`SceneComponent.K2_SetWorldRotation` (`self.ProjectileStart`) (`KismetMathLibrary.FindLookAtRotation` (`self.K2_GetActorLocation`) (`self.K2_GetActorLocation` (`GameplayStatics.GetPlayerCharacter` 0))) false false)
  (if (< _returnvalue_x _returnvalue_x_3)
    (if _returnvalue
      (`self.TurnChar` :!label _label))
    (elif (not _returnvalue)
      (goto _label))))

(event `FireAtPlayer`
  ; Shoot Projectile
  (`|SpawnActorFromClass` "/Game/Blueprints/Enemies/BP_Enemy_Projectile.BP_Enemy_Projectile_C" (`SceneComponent.K2_GetComponentToWorld` (`self.ProjectileStart`)) "Undefined" "MultiplyWithRoot" null null))

(event `self.AttackCheck.OnComponentBeginOverlap`
  (params (OverlappedComponent :type "PrimitiveComponent Object Reference") (OtherActor :type "Actor Object Reference") (OtherComp :type "PrimitiveComponent Object Reference") (OtherBodyIndex :type Integer) (bFromSweep :type Boolean) (SweepResult :type "HitResult Structure (by ref)"))
  ; AttackRangeOverlap
  (cast `/Game/Blueprints/Characters/BP_Player` OtherActor
    (:`then`
      (set `self.NotShooting` false)
      (`PaperFlipbookComponent.SetFlipbook` (`self.Sprite`) "/Game/Paperassets/FB_BeaverEnemy_Throwing.FB_BeaverEnemy_Throwing")
      (`KismetSystemLibrary.K2_SetTimer` null "TurnToPlayer" 0.05 true)
      (`KismetSystemLibrary.K2_SetTimer` null "FireAtPlayer" 1.5 true))
    (:`CastFailed`
      (`KismetSystemLibrary.PrintString` "Cant shoot this"))))

(event `self.AttackCheck.OnComponentEndOverlap`
  (params (OverlappedComponent :type "PrimitiveComponent Object Reference") (OtherActor :type "Actor Object Reference") (OtherComp :type "PrimitiveComponent Object Reference") (OtherBodyIndex :type Integer))
  ; Attack Range Broken
  (cast `/Game/Blueprints/Characters/BP_Player` OtherActor)
  (set `self.NotShooting` true)
  (`PaperFlipbookComponent.SetFlipbook` (`self.Sprite`) null)
  (`KismetSystemLibrary.K2_ClearTimer` null "TurnToPlayer")
  (`KismetSystemLibrary.K2_ClearTimer` null "FireAtPlayer"))

(event `self.ReceiveBeginPlay`
  ; Initialize Health
  (set `self.BugHP` (`self.BugMaxHP`))
  (`self.UpdateHealth`))

(event `self.ReceiveAnyDamage`
  (params (Damage :type "Float (single-precision)") (DamageType :type "DamageType Object Reference") (InstigatedBy :type "Controller Object Reference") (DamageCauser :type "Actor Object Reference"))
  ; Damage check
  (bind _output_get (set `self.BugHP` (- (`self.BugHP`) Damage)))
  (`self.UpdateHealth`)
  (if (<= _output_get 0.0)
    (`self.K2_DestroyActor`)))

(event `self.StompBox.OnComponentBeginOverlap`
  (params (OverlappedComponent :type "PrimitiveComponent Object Reference") (OtherActor :type "Actor Object Reference") (OtherComp :type "PrimitiveComponent Object Reference") (OtherBodyIndex :type Integer) (bFromSweep :type Boolean) (SweepResult :type "HitResult Structure (by ref)"))
  ; Stomp Damage
  (bind _asbp_player (cast `/Game/Blueprints/Characters/BP_Player` OtherActor))
  (`GameplayStatics.ApplyDamage` self 1.0 null _asbp_player)
  (`self.LaunchCharacter` _asbp_player (0.0 0.0 600.0) false true))

(fn `TurnChar`
  (`self.K2_SetActorRotation` (`KismetMathLibrary.ComposeRotators` (`self.K2_GetActorRotation`) (struct :`Yaw` 180.0))))

(fn `UpdateHealth`
  (return))

(fn `UserConstructionScript`)