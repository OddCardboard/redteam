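; Paper2D wolf boss that patrols, chases and charges the player, takes damage from stomps, and triggers the player's win on death.
; Tick drives movement, wall and ledge triggers turn it around, and a spotting-area timer keeps it facing the player.
; A proximity-triggered charge telegraphs, then polls overlaps to damage and knock back the player or stop on tilemaps, followed by a cooldown.
; Hits update a health-bar widget and grant brief invulnerability.
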(event `self.StompZone.OnComponentBeginOverlap`
  (params (OverlappedComponent :type "PrimitiveComponent Object Reference") (OtherActor :type "Actor Object Reference") (OtherComp :type "PrimitiveComponent Object Reference") (OtherBodyIndex :type Integer) (bFromSweep :type Boolean) (SweepResult :type "HitResult Structure (by ref)"))
  (bind (_returnvalue_x _returnvalue_y _returnvalue_z) (`KismetMathLibrary.BreakVector` (* (`KismetMathLibrary.Normal` (- (`self.K2_GetActorLocation` (`GameplayStatics.GetPlayerCharacter` 0)) (`self.K2_GetActorLocation`))) (1000.0 0.0 1000.0))))
  (bind _asbp_player (cast `/Game/Blueprints/Characters/BP_Player` OtherActor))
  (`KismetSystemLibrary.Delay` 0.1)
  (`self.LaunchCharacter` _asbp_player (`KismetMathLibrary.MakeVector` _returnvalue_x _returnvalue_y (+ _returnvalue_z 200.0)) true true)
  (`KismetSystemLibrary.Delay` 0.3)
  (`self.Damage`))

(event `self.WallCheck.OnComponentBeginOverlap`
  (params (OverlappedComponent :type "PrimitiveComponent Object Reference") (OtherActor :type "Actor Object Reference") (OtherComp :type "PrimitiveComponent Object Reference") (OtherBodyIndex :type Integer) (bFromSweep :type Boolean) (SweepResult :type "HitResult Structure (by ref)"))
  ; Terrain Checking
  (cast `/Game/Blueprints/Characters/BP_Player` OtherActor
    (:`CastFailed`
      (if (`self.IsCharging`)
        (set `self.ShouldTurn` true)
        (else
          (`self.TurnChar`))))))

(event `self.LedgeCheck.OnComponentEndOverlap`
  (params (OverlappedComponent :type "PrimitiveComponent Object Reference") (OtherActor :type "Actor Object Reference") (OtherComp :type "PrimitiveComponent Object Reference") (OtherBodyIndex :type Integer))
  ; Terrain Checking
  (cast `/Game/Blueprints/Characters/BP_Player` OtherActor
    (:`CastFailed`
      (if (`self.IsCharging`)
        (set `self.ShouldTurn` true)
        (else
          (`self.TurnChar`))))))

(event `self.ReceiveBeginPlay`
  ; Initialize Enemy
  (set `self.BossHP` (`self.BossMaxHP`))
  (`self.UpdateHealth`)
  (set `self.BossDefeated` false))

(event `self.ReceiveTick`
  (params (DeltaSeconds :type "Float (single-precision)"))
  ; Forward Movement
  (if (`self.IsCharging`)
    (if (and (not (`self.ShouldTurn`)) (not (`self.Charge Hit`)))
      (`self.AddMovementInput` (`self.GetActorForwardVector`) -6.0))
    (elif (and (not (`self.PlayerClose`)) (not (`self.IsAttacking`)))
      (`self.AddMovementInput` (`self.GetActorForwardVector`) -0.5)
      (if (`self.ShouldTurn`)
        (set `self.ShouldTurn` false)
        (`self.TurnChar`)))))

(event `self.AttackCheck.OnComponentBeginOverlap`
  (params (OverlappedComponent :type "PrimitiveComponent Object Reference") (OtherActor :type "Actor Object Reference") (OtherComp :type "PrimitiveComponent Object Reference") (OtherBodyIndex :type Integer) (bFromSweep :type Boolean) (SweepResult :type "HitResult Structure (by ref)"))
  ; Player Proximity Check
  (if (not (or (`self.IsCharging`) (`self.IsAttacking`)))
    (cast `/Game/Blueprints/Characters/BP_Player` OtherActor)
    (set `self.PlayerClose` true)))

(event `self.AttackCheck.OnComponentEndOverlap`
  (params (OverlappedComponent :type "PrimitiveComponent Object Reference") (OtherActor :type "Actor Object Reference") (OtherComp :type "PrimitiveComponent Object Reference") (OtherBodyIndex :type Integer))
  ; Player Proximity Check
  (cast `/Game/Blueprints/Characters/BP_Player` OtherActor)
  (set `self.PlayerClose` false))

(event `Damage`
  ; Damage check
  (if (not (`self.IsShielded`))
    (bind _output_get (set `self.BossHP` (- (`self.BossHP`) 1.0)))
    (`self.UpdateHealth`)
    (if (<= _output_get 0.0)
      (bind _asbp_player (cast `/Game/Blueprints/Characters/BP_Player` (`GameplayStatics.GetPlayerCharacter` 0)))
      (`/Game/Blueprints/Characters/BP_Player.GameWin` _asbp_player)
      (`GameplayStatics.PlaySound2D` "/Game/Audio/SFX/EnemyDeath.EnemyDeath" 1.0 1.0 0.0 null null)
      (`self.K2_DestroyActor`)
      (elif (not (`self.IsShielded`))
        (set `self.IsShielded` true)
        (`GameplayStatics.PlaySound2D` "/Game/Audio/SFX/hitHurtEnemy.hitHurtEnemy" 1.0 1.0 0.0 null null)
        (`KismetSystemLibrary.Delay` 1.8)
        (set `self.IsShielded` false)))))

(event `self.SpottingArea.OnComponentBeginOverlap`
  (params (OverlappedComponent :type "PrimitiveComponent Object Reference") (OtherActor :type "Actor Object Reference") (OtherComp :type "PrimitiveComponent Object Reference") (OtherBodyIndex :type Integer) (bFromSweep :type Boolean) (SweepResult :type "HitResult Structure (by ref)"))
  ; Follow Player in Area
  (if (not (`self.IsCharging`))
    (cast `/Game/Blueprints/Characters/BP_Player` OtherActor)
    (`KismetSystemLibrary.K2_SetTimer` null "ChasePlayer" 0.05 true)))

(event `self.SpottingArea.OnComponentEndOverlap`
  (params (OverlappedComponent :type "PrimitiveComponent Object Reference") (OtherActor :type "Actor Object Reference") (OtherComp :type "PrimitiveComponent Object Reference") (OtherBodyIndex :type Integer))
  ; Follow Player in Area
  (if (not (`self.IsCharging`))
    (cast `/Game/Blueprints/Characters/BP_Player` OtherActor)
    (`KismetSystemLibrary.K2_ClearTimer` null "ChasePlayer")))

(event `self.Charge Check.OnComponentBeginOverlap`
  (params (OverlappedComponent :type "PrimitiveComponent Object Reference") (OtherActor :type "Actor Object Reference") (OtherComp :type "PrimitiveComponent Object Reference") (OtherBodyIndex :type Integer) (bFromSweep :type Boolean) (SweepResult :type "HitResult Structure (by ref)"))
  ; Attack Logic
  (if (not (`self.IsCharging`))
    (cast `/Game/Blueprints/Characters/BP_Player` OtherActor)
    (`/Engine/EditorBlueprintResources/StandardMacros.DoOnce` false :!label _label
      (:`Completed`
        (`PaperFlipbookComponent.SetFlipbook` (`self.Sprite`) "/Game/Paperassets/FB_BossStandstillTeeth.FB_BossStandstillTeeth")
        (set `self.IsAttacking` true)
        (`KismetSystemLibrary.Delay` 1.0)
        (set `self.IsCharging` true)
        (`PaperFlipbookComponent.SetFlipbook` (`self.Sprite`) "/Game/Paperassets/FB_BossCharge2.FB_BossCharge2")
        (`KismetSystemLibrary.K2_ClearTimer` null "ChasePlayer")
        (`KismetSystemLibrary.K2_SetTimer` null "Charge" 0.5 true)
        ;; Cancel Charge
        (`KismetSystemLibrary.Delay` 3.0)
        (`KismetSystemLibrary.K2_ClearTimer` null "Charge")
        (set `self.IsCharging` false)
        (set `self.Charge Hit` false)
        (set `self.IsAttacking` false)
        (`PaperFlipbookComponent.SetFlipbook` (`self.Sprite`) "/Game/Paperassets/FB_BossWalk2.FB_BossWalk2")
        (`KismetSystemLibrary.K2_SetTimer` null "ChasePlayer" 0.05 true)
        (`KismetSystemLibrary.Delay` 3.0)
        (goto _label :!via `Reset`)))))

(event `ChasePlayer`
  (bind _returnvalue_x (`KismetMathLibrary.BreakVector` (`self.K2_GetActorLocation`)))
  (bind _returnvalue_x_2 (`KismetMathLibrary.BreakVector` (`self.GetActorForwardVector`)))
  (bind _returnvalue_x_3 (`KismetMathLibrary.BreakVector` (`self.K2_GetActorLocation` (`GameplayStatics.GetPlayerCharacter` 0))))
  (bind _returnvalue (== _returnvalue_x_2 1.0))
  ; ChasePlayerEvent
  (`SceneComponent.K2_SetWorldRotation` (`self.ProjectileStart`) (`KismetMathLibrary.FindLookAtRotation` (`self.K2_GetActorLocation`) (`self.K2_GetActorLocation` (`GameplayStatics.GetPlayerCharacter` 0))) false false)
  (if (< _returnvalue_x _returnvalue_x_3)
    (if _returnvalue
      (`self.TurnChar` :!label _label_2))
    (elif (not _returnvalue)
      (goto _label_2))))

(event `Charge`
  (bind (_returnvalue_x _returnvalue_y _returnvalue_z) (`KismetMathLibrary.BreakVector` (* (`KismetMathLibrary.Normal` (- (`self.K2_GetActorLocation` (`GameplayStatics.GetPlayerCharacter` 0)) (`self.K2_GetActorLocation`))) (`self.KnockbackStrength`))))
  ; Attack Logic
  ;; Charge Event
  (if (not (`self.Charge Hit`))
    (for _array_element (`PrimitiveComponent.GetOverlappingActors` (`self.AttackCheck`) null)
      (bind _asbp_player (cast `/Game/Blueprints/Characters/BP_Player` _array_element)
        (:`then`
          (set `self.Charge Hit` true)
          (`GameplayStatics.ApplyDamage` _asbp_player 1.0 null self)
          (`self.LaunchCharacter` _asbp_player (`KismetMathLibrary.MakeVector` _returnvalue_x _returnvalue_y (+ _returnvalue_z 1000.0)) false true)
          (`KismetSystemLibrary.Delay` 0.2)
          (break))
        (:`CastFailed`
          (cast `PaperTileMapActor` _array_element)
          (set `self.Charge Hit` true)
          (break))))))

(fn `TurnChar`
  (`self.K2_SetActorRotation` (`KismetMathLibrary.ComposeRotators` (`self.K2_GetActorRotation`) (struct :`Yaw` 180.0))))

(fn `UpdateHealth`
  (bind _aswidget_boss_hp (cast `/Game/Blueprints/Enemies/Widget_Boss_HP` (`WidgetComponent.GetUserWidgetObject` (`self.HealthBar`))))
  (set `/Game/Blueprints/Enemies/Widget_Boss_HP.Health` (`self.BossHP`) _aswidget_boss_hp)
  (return))

(fn `UserConstructionScript`)