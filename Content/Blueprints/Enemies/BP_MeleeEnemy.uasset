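; Melee bug enemy that patrols along its path, turning around when its wall or ledge check triggers, and dies when its health runs out.
; A spotting area starts a looping timer that turns it toward the player by comparing X positions.
; Its attack box halts movement and starts a repeating timer that bites the player.
; Stomping its top box damages it and launches the player upward; UpdateHealth is an empty stub.
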(event `self.WallCheck.OnComponentBeginOverlap`
  (params (OverlappedComponent :type "PrimitiveComponent Object Reference") (OtherActor :type "Actor Object Reference") (OtherComp :type "PrimitiveComponent Object Reference") (OtherBodyIndex :type Integer) (bFromSweep :type Boolean) (SweepResult :type "HitResult Structure (by ref)"))
  ; Terrain Checking
  (`self.TurnChar`))

(event `self.LedgeCheck.OnComponentEndOverlap`
  (params (OverlappedComponent :type "PrimitiveComponent Object Reference") (OtherActor :type "Actor Object Reference") (OtherComp :type "PrimitiveComponent Object Reference") (OtherBodyIndex :type Integer))
  ; Terrain Checking
  (`self.TurnChar`))

(event `self.ReceiveAnyDamage`
  (params (Damage :type "Float (single-precision)") (DamageType :type "DamageType Object Reference") (InstigatedBy :type "Controller Object Reference") (DamageCauser :type "Actor Object Reference"))
  ; Damage check
  (bind _output_get (set `self.BugHP` (- (`self.BugHP`) Damage)))
  (`self.UpdateHealth`)
  (if (<= _output_get 0.0)
    (`self.K2_DestroyActor`)))

(event `self.ReceiveBeginPlay`
  ; Initialize Health
  (set `self.BugHP` (`self.BugMaxHP`))
  (`self.UpdateHealth`))

(event `self.ReceiveTick`
  (params (DeltaSeconds :type "Float (single-precision)"))
  ; Forward Movement
  (if (not (`self.IsBiting`))
    (`self.AddMovementInput` (`self.GetActorForwardVector`) -1.0)))

(event `BitePlayer`
  ; BITE Player
  (for _array_element (`PrimitiveComponent.GetOverlappingActors` (`self.AttackCheck`) null)
    (bind _asbp_player (cast `/Game/Blueprints/Characters/BP_Player` _array_element))
    (`KismetSystemLibrary.PrintString` "Ouch!" true true (struct :`R` 1.0 :`A` 1.0))
    (`GameplayStatics.ApplyDamage` _asbp_player 1.0 null self)))

(event `ChasePlayer`
  (bind _returnvalue_x (`KismetMathLibrary.BreakVector` (`self.K2_GetActorLocation`)))
  (bind _returnvalue_x_2 (`KismetMathLibrary.BreakVector` (`self.GetActorForwardVector`)))
  (bind _returnvalue_x_3 (`KismetMathLibrary.BreakVector` (`self.K2_GetActorLocation` (`GameplayStatics.GetPlayerCharacter` 0))))
  (bind _returnvalue (== _returnvalue_x_2 1.0))
  ; ChasePlayerEvent
  (if (< _returnvalue_x _returnvalue_x_3)
    (if _returnvalue
      (`self.TurnChar` :!label _label))
    (elif (not _returnvalue)
      (goto _label))))

(event `self.AttackCheck.OnComponentBeginOverlap`
  (params (OverlappedComponent :type "PrimitiveComponent Object Reference") (OtherActor :type "Actor Object Reference") (OtherComp :type "PrimitiveComponent Object Reference") (OtherBodyIndex :type Integer) (bFromSweep :type Boolean) (SweepResult :type "HitResult Structure (by ref)"))
  ; AttackRangeOverlap
  (cast `/Game/Blueprints/Characters/BP_Player` OtherActor
    (:`then`
      (set `self.IsBiting` true)
      (`KismetSystemLibrary.K2_SetTimer` null "BITEPlayer" 0.4 true))
    (:`CastFailed`
      (`KismetSystemLibrary.PrintString` "Can't hit this"))))

(event `self.AttackCheck.OnComponentEndOverlap`
  (params (OverlappedComponent :type "PrimitiveComponent Object Reference") (OtherActor :type "Actor Object Reference") (OtherComp :type "PrimitiveComponent Object Reference") (OtherBodyIndex :type Integer))
  ; Attack Range Broken
  (cast `/Game/Blueprints/Characters/BP_Player` OtherActor)
  (set `self.IsBiting` false)
  (`KismetSystemLibrary.K2_ClearTimer` null "BitePlayer"))

(event `self.SpottingArea.OnComponentBeginOverlap`
  (params (OverlappedComponent :type "PrimitiveComponent Object Reference") (OtherActor :type "Actor Object Reference") (OtherComp :type "PrimitiveComponent Object Reference") (OtherBodyIndex :type Integer) (bFromSweep :type Boolean) (SweepResult :type "HitResult Structure (by ref)"))
  ; Follow Player in Area
  (cast `/Game/Blueprints/Characters/BP_Player` OtherActor)
  (`KismetSystemLibrary.K2_SetTimer` null "ChasePlayer" 0.08 true))

(event `self.SpottingArea.OnComponentEndOverlap`
  (params (OverlappedComponent :type "PrimitiveComponent Object Reference") (OtherActor :type "Actor Object Reference") (OtherComp :type "PrimitiveComponent Object Reference") (OtherBodyIndex :type Integer))
  ; Follow Player in Area
  (cast `/Game/Blueprints/Characters/BP_Player` OtherActor)
  (`KismetSystemLibrary.K2_ClearTimer` null "ChasePlayer"))

(event `self.StompBox.OnComponentBeginOverlap`
  (params (OverlappedComponent :type "PrimitiveComponent Object Reference") (OtherActor :type "Actor Object Reference") (OtherComp :type "PrimitiveComponent Object Reference") (OtherBodyIndex :type Integer) (bFromSweep :type Boolean) (SweepResult :type "HitResult Structure (by ref)"))
  ; Stomp Damage
  (bind _asbp_player (cast `/Game/Blueprints/Characters/BP_Player` OtherActor))
  (`GameplayStatics.ApplyDamage` self 1.0 null _asbp_player)
  (`self.LaunchCharacter` _asbp_player (0.0 0.0 600.0) false true))

(fn `TurnChar`
  (`self.K2_SetActorRotation` (`KismetMathLibrary.ComposeRotators` (`self.K2_GetActorRotation`) (struct :`Yaw` 180.0))))

(fn `UpdateHealth`
  (return))

(fn `UserConstructionScript`)