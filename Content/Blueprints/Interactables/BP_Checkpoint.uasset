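; A 2D platformer checkpoint that sets the player's respawn point when touched.
; When the player overlaps its box, it writes its location, offset on Y to correct the player's depth, into the game mode's SpawnTransform.
; Until flagged as up, an overlap also plays the raise flipbook, waits for its length, then switches to the raised flipbook and sets the flag.
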(event `self.ReceiveBeginPlay`
  ; Checkpoint FB Logic
  (`PaperFlipbookComponent.SetFlipbook` (`self.PaperFlipbook`) "/Game/Paperassets/FB_CheckpointDown.FB_CheckpointDown")
  (`PaperFlipbookComponent.SetLooping` (`self.PaperFlipbook`) false))

(event `self.CheckpointBox.OnComponentBeginOverlap`
  (params (OverlappedComponent :type "PrimitiveComponent Object Reference") (OtherActor :type "Actor Object Reference") (OtherComp :type "PrimitiveComponent Object Reference") (OtherBodyIndex :type Integer) (bFromSweep :type Boolean) (SweepResult :type "HitResult Structure (by ref)"))
  (bind _paperflipbook (`self.PaperFlipbook`))
  (cast `/Game/Blueprints/Characters/BP_Player` OtherActor)
  (bind _asgm_2dplatformer (cast `/Game/Blueprints/GM_2DPlatformer` (`GameplayStatics.GetGameMode`)))
  (set `/Game/Blueprints/GM_2DPlatformer.SpawnTransform` (`KismetMathLibrary.Conv_VectorToTransform` (+ (.location (`self.GetTransform`)) (0.0 10.0 0.0))) _asgm_2dplatformer)
  ; Checkpoint FB Logic
  (if (not (`self.CheckpointUp`))
    (`PaperFlipbookComponent.SetFlipbook` (`self.PaperFlipbook`) "/Game/Paperassets/FB_Checkpoint.FB_Checkpoint")
    (`PaperFlipbookComponent.PlayFromStart` _paperflipbook)
    (`KismetSystemLibrary.Delay` (`PaperFlipbookComponent.GetFlipbookLength` _paperflipbook))
    (`PaperFlipbookComponent.SetFlipbook` (`self.PaperFlipbook`) "/Game/Paperassets/FB_CheckpointUp.FB_CheckpointUp")
    (set `self.CheckpointUp` true)))

(fn `UserConstructionScript`)