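; BP_Button is a flipbook-based puzzle button that unlocks its target door when all buttons hold correct cubes.
; Overlap events on ButtonBox ignore held cubes, set the flipbook and update IsCorrectBox from the cube's IsCorrectButton flag.
; CheckAllButtons then scans every BP_Button in the level, stops at the first incorrect one, sets the door's IsUnlocked and calls UpdateDoor.
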(event `self.ButtonBox.OnComponentBeginOverlap`
  (params (OverlappedComponent :type "PrimitiveComponent Object Reference") (OtherActor :type "Actor Object Reference") (OtherComp :type "PrimitiveComponent Object Reference") (OtherBodyIndex :type Integer) (bFromSweep :type Boolean) (SweepResult :type "HitResult Structure (by ref)"))
  ; Button and Cube Collision events
  (bind _asbp_cube (cast `` OtherActor))
  (if (not (`/Game/TempHelpFolder/Interactables/BP_Button.IsHeld` _asbp_cube))
    (`PaperFlipbookComponent.SetFlipbook` (`self.RenderComponent`) null)
    (if (`/Game/TempHelpFolder/Interactables/BP_Button.IsCorrectButton` _asbp_cube)
      (set `self.IsCorrectBox` true)
      (`self.CheckAllButtons`)
      (else
        (set `self.IsCorrectBox` false)
        (`self.CheckAllButtons`)))))

(event `self.ButtonBox.OnComponentEndOverlap`
  (params (OverlappedComponent :type "PrimitiveComponent Object Reference") (OtherActor :type "Actor Object Reference") (OtherComp :type "PrimitiveComponent Object Reference") (OtherBodyIndex :type Integer))
  ; Button and Cube Collision events
  (bind _asbp_cube (cast `` OtherActor))
  (if (not (`/Game/TempHelpFolder/Interactables/BP_Button.IsHeld` _asbp_cube))
    (`PaperFlipbookComponent.SetFlipbook` (`self.RenderComponent`) null)
    (if (`/Game/TempHelpFolder/Interactables/BP_Button.IsCorrectButton` _asbp_cube)
      (set `self.IsCorrectBox` false)
      (`self.CheckAllButtons`))))

(event `CheckAllButtons`
  (bind (_targetdoor _targetdoor_2) (`self.TargetDoor`))
  ; Checks if ALL buttons overlap with the correct Cube
  (bind _outactors (`GameplayStatics.GetAllActorsOfClass` "BP_Button_C"))
  (for _array_element _outactors
    (if (`/Game/TempHelpFolder/Interactables/BP_Button.IsCorrectBox` _array_element)
      (set `self.AllButtonsTrue` true)
      (else
        (set `self.AllButtonsTrue` false)
        (break))))
  (if (`self.AllButtonsTrue`)
    (`KismetSystemLibrary.PrintString` "ALL TRUE")
    (set `/Game/TempHelpFolder/Interactables/BP_Button.IsUnlocked` true _targetdoor_2)
    (else
      (set `/Game/TempHelpFolder/Interactables/BP_Button.IsUnlocked` false _targetdoor_2)))
  (`self.UpdateDoor` _targetdoor_2))

(fn `UserConstructionScript`)